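; BP_RangedAI is a ranged enemy character that shoots projectiles and is driven through an AI Blackboard.
; Its AttackRange overlap sets the ReadytoAttack key when BP_ThirdPersonCharacter enters and clears it on exit.
; ShootingAttack spawns a scaled BP_Projectile at ProjectileSpawn; it and range entry raise an animation flag, which no live logic here resets.
; UpdateWalkSpeed exposes a setter for maximum walk speed.
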(event `ShootingAttack`
  (bind (_returnvalue_location _returnvalue_rotation) (`KismetMathLibrary.BreakTransform` (`SceneComponent.K2_GetComponentToWorld` (`self.ProjectileSpawn`))))
  ;[1 1 1] Ranged attack function needs BT_Projectile to work
  (`|SpawnActorFromClass` "/Game/AI_BP/RangedEnemy/Projectile/BP_Projectile.BP_Projectile_C" (`KismetMathLibrary.MakeTransform` _returnvalue_location _returnvalue_rotation (0.15 0.1 0.09)) "AlwaysSpawn" "OverrideRootScale" null null)
  (set `self.IsAttackingForAnim` true) ; Boolean responsible foranimation
)

(event `self.attack range.OnComponentBeginOverlap`
  (params (OverlappedComponent :type "PrimitiveComponent Object Reference") (OtherActor :type "Actor Object Reference") (OtherComp :type "PrimitiveComponent Object Reference") (OtherBodyIndex :type Integer) (bFromSweep :type Boolean) (SweepResult :type "HitResult Structure (by ref)"))
  (cast `/Game/ThirdPerson/Blueprints/BP_ThirdPersonCharacter` OtherActor)
  (`KismetSystemLibrary.PrintString` "iSwORKING")
  (`BlackboardComponent.SetValueAsBool` (`AIBlueprintHelperLibrary.GetBlackboard` null) "ReadytoAttack" true)
  (set `self.IsAttackingForAnim` true))

(event `self.attack range.OnComponentEndOverlap`
  (params (OverlappedComponent :type "PrimitiveComponent Object Reference") (OtherActor :type "Actor Object Reference") (OtherComp :type "PrimitiveComponent Object Reference") (OtherBodyIndex :type Integer))
  (cast `/Game/ThirdPerson/Blueprints/BP_ThirdPersonCharacter` OtherActor)
  (`KismetSystemLibrary.PrintString` "iSwORKING")
  (`BlackboardComponent.SetValueAsBool` (`AIBlueprintHelperLibrary.GetBlackboard` null) "ReadytoAttack" false))

(fn `UpdateWalkSpeed`
  (params (NewWalkSpeed :type "Float (double-precision)"))
  (set `CharacterMovementComponent.MaxWalkSpeed` NewWalkSpeed (`self.CharacterMovement`)))

(fn `UserConstructionScript`)